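; Road segment actor for an endless-road game, with car obstacles that trigger timed quick-time events.
; On BeginPlay it reads difficulty from Kachow_GI to set spawn odds and QTE duration, then after a delay may reveal one of four cars.
; Hitting a car starts a keyed QTE on the player; passing it hides that car.
; Its trigger asks the game mode to add another road, then destroys this one after a delay.
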(event OnComponentBeginOverlap(GenerationCollider)
  (params (OverlappedComponent :type Primitive%20Component%20Object%20Reference) (OtherActor :type Actor%20Object%20Reference) (OtherComp :type Primitive%20Component%20Object%20Reference) (OtherBodyIndex :type Integer) (bFromSweep :type Boolean) (SweepResult :type Hit%20Result%20Structure%20%28by%20ref%29))
  ;[1 1 1] Create New Road Bit
  (Utilities|Casting|CastToBP_ThirdPersonCharacter OtherActor)
  (bind _asbp_third_person_game_mode (Utilities|Casting|CastToBP_ThirdPersonGameMode (Game|GetGameMode)))
  (Default|AddRoad _asbp_third_person_game_mode)
  (if true
    (Utilities|FlowControl|Delay 5.0)
    (Actor|DestroyActor)))

(event OnComponentHit(PinkCar)
  (params (HitComponent :type Primitive%20Component%20Object%20Reference) (OtherActor :type Actor%20Object%20Reference) (OtherComp :type Primitive%20Component%20Object%20Reference) (NormalImpulse :type Vector :default "0, 0, 0") (Hit :type Hit%20Result%20Structure%20%28by%20ref%29))
  (bind _returnvalue (Game|GetPlayerController 0))
  (bind _returnvalue_2 (Pawn|GetControlledPawn _returnvalue))
  ;[1 1 1] Overlap
  (if (== OtherActor _returnvalue_2)
    (Variables|Default|SetPink%20Car%20hit true)
    (bind _asbp_third_person_character (Utilities|Casting|CastToBP_ThirdPersonCharacter _returnvalue_2))
    (Default|CreateQTEEvent _asbp_third_person_character "One" "1" true (Variables|Default|GetQTE%20Duration) self)))

(event OnComponentHit(OrangeCar)
  (params (HitComponent :type Primitive%20Component%20Object%20Reference) (OtherActor :type Actor%20Object%20Reference) (OtherComp :type Primitive%20Component%20Object%20Reference) (NormalImpulse :type Vector :default "0, 0, 0") (Hit :type Hit%20Result%20Structure%20%28by%20ref%29))
  (bind _returnvalue (Game|GetPlayerController 0))
  (bind _returnvalue_2 (Pawn|GetControlledPawn _returnvalue))
  ;[1 1 1] Overlap
  (if (== OtherActor _returnvalue_2)
    (Variables|Default|SetOrange%20Car%20hit true)
    (bind _asbp_third_person_character (Utilities|Casting|CastToBP_ThirdPersonCharacter _returnvalue_2))
    (Default|CreateQTEEvent _asbp_third_person_character "Two" "2" true (Variables|Default|GetQTE%20Duration) self)))

(event OnComponentHit(PinkCar1)
  (params (HitComponent :type Primitive%20Component%20Object%20Reference) (OtherActor :type Actor%20Object%20Reference) (OtherComp :type Primitive%20Component%20Object%20Reference) (NormalImpulse :type Vector :default "0, 0, 0") (Hit :type Hit%20Result%20Structure%20%28by%20ref%29))
  (bind _returnvalue (Game|GetPlayerController 0))
  (bind _returnvalue_2 (Pawn|GetControlledPawn _returnvalue))
  ;[1 1 1] Overlap
  (if (== OtherActor _returnvalue_2)
    (Variables|Default|SetPink%20Car1%20hit true)
    (bind _asbp_third_person_character (Utilities|Casting|CastToBP_ThirdPersonCharacter _returnvalue_2))
    (Default|CreateQTEEvent _asbp_third_person_character "Three" "3" true (Variables|Default|GetQTE%20Duration) self)))

(event OnComponentHit(OrangeCar1)
  (params (HitComponent :type Primitive%20Component%20Object%20Reference) (OtherActor :type Actor%20Object%20Reference) (OtherComp :type Primitive%20Component%20Object%20Reference) (NormalImpulse :type Vector :default "0, 0, 0") (Hit :type Hit%20Result%20Structure%20%28by%20ref%29))
  (bind _returnvalue (Game|GetPlayerController 0))
  (bind _returnvalue_2 (Pawn|GetControlledPawn _returnvalue))
  ;[1 1 1] Overlap
  (if (== OtherActor _returnvalue_2)
    (Variables|Default|SetOrange%20Car1%20hit true)
    (bind _asbp_third_person_character (Utilities|Casting|CastToBP_ThirdPersonCharacter _returnvalue_2))
    (Default|CreateQTEEvent _asbp_third_person_character "Four" "4" true (Variables|Default|GetQTE%20Duration) self)))

(event EventBeginPlay
  (bind _pink_car (Variables|Default|GetPink%20Car))
  (bind _pink_car1 (Variables|Default|GetPink%20Car1))
  (bind _orange_car (Variables|Default|GetOrange%20Car))
  (bind _orange_car1 (Variables|Default|GetOrange%20Car1))
  ;[1 1 1] Make Obsticles appear
  (bind _askachow_gi (Utilities|Casting|CastToKachow_GI (Game|GetGameInstance)))
  (if (Variables|/Game/All_Used_Items/Kachow_GI.Kachow_GI_C|GetEasyMode _askachow_gi)
    (Variables|Default|SetMaxRange 15)
    (Variables|Default|SetQTE%20Duration 2e+01)
    (elif (Variables|/Game/All_Used_Items/Kachow_GI.Kachow_GI_C|GetMedMode _askachow_gi)
      (Variables|Default|SetMaxRange 10)
      (Variables|Default|SetQTE%20Duration 9.0)
      (elif (Variables|/Game/All_Used_Items/Kachow_GI.Kachow_GI_C|GetHardMode _askachow_gi)
        (Variables|Default|SetMaxRange 4)
        (Variables|Default|SetQTE%20Duration 4.0)
        (else
          (Variables|Default|SetMaxRange 8)
          (Variables|Default|SetQTE%20Duration 1e+01)))))
  (Utilities|FlowControl|Delay 4.0)
  (switch int (Math|Random|RandomIntegerinRange 0 (Variables|Default|GetMaxRange))
    (:0
      (Rendering|SetVisibility _pink_car true false)
      (Collision|SetCollisionEnabled _pink_car "QueryAndPhysics")
      (Components|Tick|SetComponentTickEnabled _pink_car true))
    (:1
      (Rendering|SetVisibility _pink_car1 true false)
      (Collision|SetCollisionEnabled _pink_car1 "QueryAndPhysics")
      (Components|Tick|SetComponentTickEnabled _pink_car1 true))
    (:2
      (Rendering|SetVisibility _orange_car true false)
      (Collision|SetCollisionEnabled _orange_car "QueryAndPhysics")
      (Components|Tick|SetComponentTickEnabled _orange_car true))
    (:3
      (Rendering|SetVisibility _orange_car1 true false)
      (Collision|SetCollisionEnabled _orange_car1 "QueryAndPhysics")
      (Components|Tick|SetComponentTickEnabled _orange_car1 true))))

(event EventQtePassedScript
  (bind _pink_car (Variables|Default|GetPink%20Car))
  (bind _orange_car (Variables|Default|GetOrange%20Car))
  (bind _pink_car1 (Variables|Default|GetPink%20Car1))
  (bind _orange_car1 (Variables|Default|GetOrange%20Car1))
  ;[1 1 1] QTE Passed
  (if (Variables|Default|GetPink%20Car%20hit)
    (Rendering|SetVisibility _pink_car false false)
    (Collision|SetCollisionEnabled _pink_car "NoCollision")
    (Components|Tick|SetComponentTickEnabled _pink_car true)
    (elif (Variables|Default|GetOrange%20Car%20hit)
      (Rendering|SetVisibility _orange_car false false)
      (Collision|SetCollisionEnabled _orange_car "NoCollision")
      (Components|Tick|SetComponentTickEnabled _orange_car true)
      (elif (Variables|Default|GetPink%20Car1%20hit)
        (Rendering|SetVisibility _pink_car1 false false)
        (Collision|SetCollisionEnabled _pink_car1 "NoCollision")
        (Components|Tick|SetComponentTickEnabled _pink_car1 true)
        (elif (Variables|Default|GetOrange%20Car1%20hit)
          (Rendering|SetVisibility _orange_car1 false false)
          (Collision|SetCollisionEnabled _orange_car1 "NoCollision")
          (Components|Tick|SetComponentTickEnabled _orange_car1 true))))))

(fn ConstructionScript)

(fn GetArrowTransform
  (return (Transformation|GetWorldTransform (Variables|Default|GetArrow))))